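; DPdrawer is an interactable drawer that the player character can get into and out of.
; Each Interact event flips an Inside flag and teleports player 0 to the location and rotation of the REFInside or REFOutside reference component.
; The Door's relative rotation snaps closed on entry and swings open on exit, with no animation.
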(event EventBeginPlay)

(event Collision|EventActorBeginOverlap
  (params (OtherActor :type Actor%20Object%20Reference)))

(event EventTick
  (params (DeltaSeconds :type Float%20%28single-precision%29)))

(event EventInteract
  (bind _ref_inside (Variables|Default|GetREF%20inside))
  (bind _ref_outside (Variables|Default|GetREF%20outside))
  (bind _returnvalue (Transformation|GetWorldTransform _ref_inside))
  (bind _returnvalue_2 (Transformation|GetWorldTransform _ref_outside))
  (if (not (Variables|Default|Getinside))
    (Variables|Default|Setinside true)
    (Transformation|SetActorTransform (Game|GetPlayerCharacter 0) (Math|Transform|MakeTransform (.location _returnvalue) (.rotation _returnvalue) "1.000000,1.000000,1.000000"))
    (Transformation|SetRelativeRotation (Variables|Default|Getdoor) "0, 0, 0" false false)
    (else
      (Variables|Default|Setinside false)
      (Transformation|SetActorTransform (Game|GetPlayerCharacter 0) (Math|Transform|MakeTransform (.location _returnvalue_2) (.rotation _returnvalue_2) "1.000000,1.000000,1.000000"))
      (Transformation|SetRelativeRotation (Variables|Default|Getdoor) "0.000000,109.000000,0.000000" false false))))

(fn ConstructionScript)